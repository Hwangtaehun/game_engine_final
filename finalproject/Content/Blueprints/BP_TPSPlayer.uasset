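; Player Blueprint for a third-person shooter that connects the character to its HUD and game-over screen.
; BeginPlay creates the UI_Screen widget, then after a brief delay fills the HP ratio and text and sets the non-grenade weapon display.
; OnUsingGrenade pushes the grenade flag to the HUD and triggers its weapon swap.
; OnGameOver runs the parent logic, shows the mouse cursor and adds UI_GameOver.
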(event `self.ReceiveBeginPlay`
  (bind _returnvalue (`|CreateWidget` "/Game/UI/UI_Screen.UI_Screen_C" (`GameplayStatics.GetPlayerController` 0)))
  (bind _output_get (set `self.UI_Screen` _returnvalue))
  (`UserWidget.AddToViewport` _output_get 0)
  (`KismetSystemLibrary.Delay` 0.05)
  (`self.UIctrlHP`)
  (`self.OnUsingGrenade` false))

(event `self.OnUsingGrenade`
  (params (isGrenade :type Boolean))
  (bind _ui_screen (`self.UI_Screen`))
  (`/Engine/EditorBlueprintResources/StandardMacros.IsValid` _ui_screen
    (:`Is Valid`
      (set `/Game/UI/UI_Screen.isGrenaded` isGrenade _ui_screen)
      (`/Game/UI/UI_Screen.SwapWeapon` _ui_screen))))

(event `self.OnGameOver`
  (`parent.OnGameOver`)
  (set `PlayerController.bShowMouseCursor` true (`GameplayStatics.GetPlayerController` 0))
  (bind _returnvalue (`|CreateWidget` "/Game/UI/UI_GameOver.UI_GameOver_C"))
  (`UserWidget.AddToViewport` _returnvalue 0))

(fn `UIctrlHP`
  (bind _hp (`self.hp`))
  (bind _initialhp (`self.initialHp`))
  (bind _ui_screen (`self.UI_Screen`))
  (set `/Game/UI/UI_Screen.hpRatio` (/ _hp _initialhp) _ui_screen)
  (set `/Game/UI/UI_Screen.hpString` (`KismetStringLibrary.Concat_StrStr` (`KismetStringLibrary.Conv_IntToString` _hp) "/" (`KismetStringLibrary.Conv_IntToString` _initialhp)) _ui_screen))

(fn `UserConstructionScript`)